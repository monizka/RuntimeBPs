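; Function library for a runtime Blueprint graph editor, covering pin colors, connection rules and value defaults.
; GetVariableColor maps each variable type to primary and secondary colors.
; CheckVariableConversion finds a conversion node by filtering node class names and matching class-default pin types, while CheckVariableInheritance permits child-to-parent object connections through a hard-coded type hierarchy.
; Small helpers parse bool strings and reset values when their type changes.
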(fn GetVariableColor
  (params (VariableType :type EVariableTypes%20Enum :default "Bool"))
  (bind _returnvalue (Math|Color|MakeColor 0.0 0.401978 0.913099))
  (bind _returnvalue_2 (Math|Color|MakeColor 0.122139 0.473532 0.913099))
  (return (Utilities|Select :Index VariableType :Bool "(R=0.300544,G=0.000000,B=0.000000,A=1.000000)" :Byte "(R=0.000000,G=0.158961,B=0.130136,A=1.000000)" :Int "(R=0.012983,G=0.775822,B=0.428691,A=1.000000)" :Float "(R=0.356400,G=1.000000,B=0.059511,A=1.000000)" :Name "(R=0.611765,G=0.223529,B=1.000000,A=1.000000)" :String "(R=1.000000,G=0.000000,B=0.666667,A=1.000000)" :Text "(R=0.807843,G=0.200000,B=0.400000,A=1.000000)" :Vector "(R=1.000000,G=0.592157,B=0.015686,A=1.000000)" :Rotator "(R=0.356863,G=0.454902,B=1.000000,A=1.000000)" :Transform "(R=1.000000,G=0.168627,B=0.000000,A=1.000000)" :Vector2D "(R=0.039216,G=0.090196,B=0.603922,A=1.000000)" :Vector4 "(R=0.466667,G=0.039216,B=0.000000,A=1.000000)" :LinearColor "(R=0.001821,G=0.012983,B=0.323143,A=1.000000)" :IntVector "(R=0.000000,G=0.806952,B=0.768151,A=1.000000)" :IntVector4 "(R=0.003922,G=0.254902,B=0.356863,A=1.000000)" :HitResult "(R=0.080786,G=0.089205,B=0.323143,A=1.000000)" :Object "(R=0.000000,G=0.401978,B=0.913099,A=1.000000)" :Actor _returnvalue :PlayerController _returnvalue :Pawn _returnvalue :Character _returnvalue :SceneComponent _returnvalue :PrimitiveComponent _returnvalue :StaticMeshComponent _returnvalue :LightComponent _returnvalue :ParticleSystemComponent _returnvalue :DamageType _returnvalue :Class "(R=0.107023,G=0.002428,B=0.485150,A=1.000000)" :StaticMesh _returnvalue_2 :MaterialInterface _returnvalue_2 :ParticleSystem _returnvalue_2 :Exec "(R=1.000000,G=1.000000,B=1.000000,A=1.000000)" :WildCard "(R=0.453125,G=0.453125,B=0.453125,A=1.000000)") (Utilities|Select :Index VariableType :Bool "(R=0.300544,G=0.000000,B=0.000000,A=1.000000)" :Byte "(R=0.000000,G=0.158961,B=0.130136,A=1.000000)" :Int "(R=0.012983,G=0.775822,B=0.428691,A=1.000000)" :Float "(R=0.356400,G=1.000000,B=0.059511,A=1.000000)" :Name "(R=0.611765,G=0.223529,B=1.000000,A=1.000000)" :String "(R=1.000000,G=0.000000,B=0.666667,A=1.000000)" :Text "(R=0.807843,G=0.200000,B=0.400000,A=1.000000)" :Vector "(R=1.000000,G=0.592157,B=0.015686,A=1.000000)" :Rotator "(R=0.356863,G=0.454902,B=1.000000,A=1.000000)" :Transform "(R=1.000000,G=0.168627,B=0.000000,A=1.000000)" :Vector2D "(R=0.039216,G=0.090196,B=0.603922,A=1.000000)" :Vector4 "(R=0.466667,G=0.039216,B=0.000000,A=1.000000)" :LinearColor "(R=0.001821,G=0.012983,B=0.323143,A=1.000000)" :IntVector "(R=0.000000,G=0.806952,B=0.768151,A=1.000000)" :IntVector4 "(R=0.003922,G=0.254902,B=0.356863,A=1.000000)" :HitResult "(R=0.001821,G=0.012983,B=0.323143,A=1.000000)" :Object "(R=0.000000,G=0.401978,B=0.913099,A=1.000000)" :Actor "(R=0.000000,G=0.029557,B=0.822786,A=1.000000)" :PlayerController "(R=0.000000,G=1.000000,B=0.784756,A=1.000000)" :Pawn "(R=1.000000,G=1.000000,B=1.000000,A=1.000000)" :Character "(R=0.000000,G=1.000000,B=0.122092,A=1.000000)" :SceneComponent "(R=0.000000,G=0.029557,B=0.822786,A=1.000000)" :PrimitiveComponent "(R=0.000000,G=0.371553,B=0.822786,A=1.000000)" :StaticMeshComponent "(R=1.000000,G=0.300544,B=0.300544,A=1.000000)" :LightComponent "(R=0.343828,G=0.815000,B=0.804776,A=1.000000)" :ParticleSystemComponent "(R=0.291771,G=0.291771,B=1.000000,A=1.000000)" :DamageType _returnvalue :Class "(R=0.107023,G=0.002428,B=0.485150,A=1.000000)" :StaticMesh "(R=1.000000,G=0.300544,B=0.300544,A=1.000000)" :MaterialInterface "(R=0.975468,G=1.000000,B=0.300000,A=1.000000)" :ParticleSystem "(R=0.291771,G=0.291771,B=1.000000,A=1.000000)" :Exec "(R=1.000000,G=1.000000,B=1.000000,A=1.000000)" :WildCard "(R=0.453125,G=0.453125,B=0.453125,A=1.000000)")))

(fn StringtoBool
  (params (InString :type String))
  (return (Utilities|Enum|Equal(Enum) InString "true")))

(fn CheckVariableConversion
  (params (EditorGraph :type BP%20Editor%20Graph%20Object%20Reference) (InputPin :type Input%20Pin%20Object%20Reference) (OutputPin :type Input%20Pin%20Object%20Reference))
  (bind _array_element (Utilities|Array|ForEachLoopwithBreak (Variables|/Game/RuntimeBlueprints/Widgets/BPEditorGraph.BPEditorGraph_C|GetBPNodeClasses EditorGraph) :!label _label)
    (:LoopBody
      (bind _asruntime_bp_object (Utilities|Casting|CastToRuntimeBpObjectClass _array_element))
      (if (Math|Boolean|ORBoolean (Utilities|String|Contains (Utilities|GetClassDisplayName _asruntime_bp_object) "Conv_") (Utilities|String|Contains (Utilities|GetClassDisplayName _asruntime_bp_object) "Trunc") (Utilities|String|Contains (Utilities|GetClassDisplayName _asruntime_bp_object) "XVector"))
        (if (and (Utilities|Enum|Equal(Enum) (Variables|/Game/RuntimeBlueprints/Widgets/Nodes/InputPin.InputPin_C|GetVariableType OutputPin) (Utilities|Struct|BreakPinStruct (Utilities|Array|Get(acopy) (.InputPins (Utilities|GetClassDefaults _asruntime_bp_object))))) (Utilities|Enum|Equal(Enum) (Variables|/Game/RuntimeBlueprints/Widgets/Nodes/InputPin.InputPin_C|GetVariableType InputPin) (Utilities|Struct|BreakPinStruct (Utilities|Array|Get(acopy) (.OutputPins (Utilities|GetClassDefaults _asruntime_bp_object))))))
          (LocalVariables|SetNode _asruntime_bp_object)
          (goto _label Break))))
    (:Completed
      (return (LocalVariables|GetNode) (Utilities|IsValidClass (LocalVariables|GetNode))))))

(fn CheckVariableInheritance
  (params (InputPin :type Input%20Pin%20Object%20Reference) (OutputPin :type Input%20Pin%20Object%20Reference))
  (bind _variabletype (Variables|/Game/RuntimeBlueprints/Widgets/Nodes/InputPin.InputPin_C|GetVariableType OutputPin))
  (Utilities|FlowControl|Sequence
    (:then_0
      (switch Utilities|FlowControl|Switch|SwitchonEVariableTypes (Variables|/Game/RuntimeBlueprints/Widgets/Nodes/InputPin.InputPin_C|GetVariableType InputPin)
        (:Object
          (switch Utilities|FlowControl|Switch|SwitchonEVariableTypes _variabletype
            (:Object
              _)
            (:Actor
              _)
            (:PlayerController
              _)
            (:Pawn
              _)
            (:Character
              _)
            (:SceneComponent
              _)
            (:PrimitiveComponent
              _)
            (:StaticMeshComponent
              _)
            (:LightComponent
              _)
            (:ParticleSystemComponent
              _)
            (:DamageType
              _))
          (LocalVariables|SetConnect true))
        (:Actor
          (switch Utilities|FlowControl|Switch|SwitchonEVariableTypes _variabletype
            (:Actor
              _)
            (:PlayerController
              _)
            (:Pawn
              _)
            (:Character
              _))
          (LocalVariables|SetConnect true))
        (:Pawn
          (switch Utilities|FlowControl|Switch|SwitchonEVariableTypes _variabletype
            (:Pawn
              _)
            (:Character
              _))
          (LocalVariables|SetConnect true))
        (:SceneComponent
          (switch Utilities|FlowControl|Switch|SwitchonEVariableTypes _variabletype
            (:SceneComponent
              _)
            (:StaticMeshComponent
              _)
            (:LightComponent
              _)
            (:ParticleSystemComponent
              _))
          (LocalVariables|SetConnect true))
        (:PrimitiveComponent
          (switch Utilities|FlowControl|Switch|SwitchonEVariableTypes _variabletype
            (:PrimitiveComponent
              _)
            (:StaticMeshComponent
              _)
            (:ParticleSystemComponent
              _))
          (LocalVariables|SetConnect true))))
    (:then_1
      (return (LocalVariables|GetConnect)))))

(fn ChangeValueArg
  (params (Values :type Array%20of%20Node%20Var%20Args%20Structures) (NewVariableType :type EVariableTypes%20Enum :default "Bool") (Array :type Boolean))
  (Utilities|FlowControl|Sequence
    (:then_0
      (Class|RuntimeBpLibrary|SetDefaultArg Values NewVariableType))
    (:then_1
      (if Array
        (Class|RuntimeBpLibrary|ClearNodeVarArgs Values NewVariableType Array)))))